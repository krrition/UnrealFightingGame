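; Animation notify for the Atk3 attack that deals fixed damage to actors inside a box at the Atk3Socket of the sequence render component.
; With a valid owning instance, it runs a box overlap with an empty object-type filter, ignores the owner, then damages and prints each hit actor.
; Without one, it draws the box as a debug shape instead.
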(event EventOnReceiveNotify
  (params (OwningInstance :type Paper%20ZD%20Anim%20Instance%20Object%20Reference))
  (bind _sequencerendercomponent (Variables|Default|GetSequenceRenderComponent))
  (bind _boxsize (Variables|Default|GetBoxSize))
  (bind _returnvalue (Transformation|GetSocketLocation _sequencerendercomponent "Atk3Socket"))
  (Utilities|IsValid OwningInstance
    (:Is%20Valid
      (bind _outactors (Collision|BoxOverlapActors _returnvalue _boxsize (Utilities|Array|MakeArray) 0 (Utilities|Array|MakeArray (Class|PaperZDAnimInstance|GetOwningActor OwningInstance)) :!class /Script/Engine.KismetSystemLibrary))
      (for _array_element _outactors
        (Development|PrintString (Utilities|GetDisplayName _array_element))
        (Game|Damage|ApplyDamage _array_element 1e+01 0 0))
      (Development|PrintString "no more actors"))
    (:Is%20Not%20Valid
      (Rendering|Debug|DrawDebugBox _returnvalue _boxsize "(R=1.000000,G=0.883412,B=0.000000,A=1.000000)" "0, 0, 0" 0.0 5.0))))