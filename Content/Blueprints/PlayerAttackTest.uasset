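; Test 2D player Blueprint for flipbook-animated X-axis movement, combo attacks and blocking.
; Tick stores the current flipbook's name as the state, which StateCheck uses to gate movement, attack and damage logic.
; Attack inputs open timed link flags for combos or call PlayAnim, which jumps animation nodes behind a DoOnce lockout lasting flipbook length plus delay.
; Blocking requires GetDown while idle or walking; block and damage results only print.
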(event Input|EnhancedActionEvents|EnhancedInputActionMove_IA
  (params (ActionValue :type Float%20%28double-precision%29) (ElapsedSeconds :type Float%20%28double-precision%29) (TriggeredSeconds :type Float%20%28double-precision%29) (InputAction :type Input%20Action%20Object%20Reference :default "/Game/Inputs/Move_IA.Move_IA"))
  ;[1 1 1] Start Movement With Acceleration
  (Utilities|StateCheck "Walk"
    (:Same
      (Pawn|Input|AddMovementInput "1.000000,0.000000,0.000000" (* ActionValue (Variables|Default|GetMoveMultiplier)) false))
    (:Different
      (Utilities|StateCheck "Idle"
        (:Same
          (Pawn|Input|AddMovementInput "1.000000,0.000000,0.000000" (* ActionValue 0.1) false))))))

(event Input|EnhancedActionEvents|EnhancedInputActionAttack1_IA
  (params (ActionValue :type Boolean) (ElapsedSeconds :type Float%20%28double-precision%29) (TriggeredSeconds :type Float%20%28double-precision%29) (InputAction :type Input%20Action%20Object%20Reference :default "/Game/Inputs/Attack1_IA.Attack1_IA"))
  ;[1 1 1] Attack and Delay
  (Utilities|StateCheck "Attack2"
    (:Different
      (Utilities|PlayAnim "StringA1" 0.2))))

(event Input|EnhancedActionEvents|EnhancedInputActionAttack2_IA
  (params (ActionValue :type Boolean) (ElapsedSeconds :type Float%20%28double-precision%29) (TriggeredSeconds :type Float%20%28double-precision%29) (InputAction :type Input%20Action%20Object%20Reference :default "/Game/Inputs/Attack2_IA.Attack2_IA"))
  ;[1 1 1] Links and Other Strings
  (Utilities|StateCheck "Attack1"
    (:Same
      (Variables|Default|SetAttack2Link true)
      (Utilities|FlowControl|Delay 0.2)
      (Variables|Default|SetAttack2Link false))
    (:Different
      (Utilities|StateCheck "Idle"
        (:Same
          _)
        (:Different
          (Utilities|StateCheck "Walk"
            (:Same
              _))))
      (Utilities|PlayAnim "StringA2" 0.2))))

(event Input|EnhancedActionEvents|EnhancedInputActionAttack3_IA
  (params (ActionValue :type Boolean) (ElapsedSeconds :type Float%20%28double-precision%29) (TriggeredSeconds :type Float%20%28double-precision%29) (InputAction :type Input%20Action%20Object%20Reference :default "/Game/Inputs/Attack3_IA.Attack3_IA"))
  ;[1 1 1] Links and Other Strings
  (:Completed
    (Utilities|StateCheck "Attack2"
      (:Same
        (Variables|Default|SetAttack3Link true)
        (Utilities|FlowControl|Delay 0.5)
        (Variables|Default|SetAttack3Link false))
      (:Different
        (Utilities|PlayAnim "SpecialA" 0.4)))))

(event EventBeginPlay
  ;[1 1 1] Mapping Context
  (bind _asplayer_controller (Utilities|Casting|CastToPlayerController (Pawn|GetController)))
  (Input|AddMappingContext (PlayerController|LocalPlayerSubsystems|GetEnhancedInputLocalPlayerSubsystem _asplayer_controller) "/Game/Inputs/DirectionInputs.DirectionInputs" 0 "(bIgnoreAllPressedKeysUntilRelease=True,bForceImmediately=False,bNotifyUserSettings=False)"))

(event Collision|EventActorBeginOverlap
  (params (OtherActor :type Actor%20Object%20Reference)))

(event EventTick
  (params (DeltaSeconds :type Float%20%28single-precision%29))
  ;[1 1 1] Set State
  (CallFunction|CurrentState))

(event Game|Damage|EventAnyDamage
  (params (Damage :type Float%20%28single-precision%29) (DamageType :type Damage%20Type%20Object%20Reference) (InstigatedBy :type Controller%20Object%20Reference) (DamageCauser :type Actor%20Object%20Reference))
  ;[1 1 1] Blocking and Taking Damage
  (Utilities|StateCheck "Idle"
    (:Same
      (if (Input|EnhancedActionValues|GetDown) :!label _label
        (Development|PrintString "Block")
        (else
          (Development|PrintString "Damage Taken" :!label _label_2))))
    (:Different
      (Utilities|StateCheck "Walk"
        (:Same
          (goto _label))
        (:Different
          (goto _label_2))))))

(fn ConstructionScript)

(fn RestartAnim
  (Components|Timeline|SetLooping (Variables|Default|GetSprite) true)
  (if (not (Audio|Components|Audio|IsPlaying (Variables|Default|GetSprite)))
    (Audio|Components|Audio|Play (Variables|Default|GetSprite))))

(fn HitCheck)

(fn CurrentState
  (Variables|Default|SetState (Utilities|GetDisplayName (Class|PaperFlipbookComponent|GetFlipbook (Variables|Default|GetSprite)))))