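; TargetBox is a test target actor that reacts to hits from PlayerAttackTest.
; On overlap it prints a debug message and compares the other actor to that class instance's OverHit and ForHit references.
; Each match snaps the Cube component to its own fixed tilted world rotation, with no reset.
; Any damage received is only printed to screen.
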(event EventBeginPlay)

(event EventTick
  (params (DeltaSeconds :type Float%20%28single-precision%29)))

(event Collision|EventActorBeginOverlap
  (params (OtherActor :type Actor%20Object%20Reference))
  (bind _cube (Variables|Default|GetCube))
  (Development|PrintString "Hit")
  (bind _returnvalue (Actor|GetActorOfClass "/Game/Blueprints/PlayerAttackTest.PlayerAttackTest_C"))
  (if (== OtherActor (Variables|/Game/Blueprints/PlayerAttackTest.PlayerAttackTest_C|GetOver%20Hit _returnvalue))
    (Transformation|SetWorldRotation _cube "-45.000000,0.000000,0.000000" false false)
    (elif (== OtherActor (Variables|/Game/Blueprints/PlayerAttackTest.PlayerAttackTest_C|GetFor%20Hit _returnvalue))
      (Transformation|SetWorldRotation _cube "0.000000,0.000000,45.000000" false false))))

(event Game|Damage|EventAnyDamage
  (params (Damage :type Float%20%28single-precision%29) (DamageType :type Damage%20Type%20Object%20Reference) (InstigatedBy :type Controller%20Object%20Reference) (DamageCauser :type Actor%20Object%20Reference))
  (Development|PrintString (Utilities|String|ToString(Float) Damage)))

(fn ConstructionScript)